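; GA_Protect is a Gameplay Ability that applies the GE_Protect effect to its owner and plays a protect montage.
; On activation it uses the GAS_Tarea3Character's IsAttacking flag as a guard: if already set, it clears the flag and ends.
; Otherwise it sets the flag, self-applies the effect and plays AM_Protect at AnimSpeed.
; Only montage completion clears the flag and ends the ability; interruption is not handled.
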(event `self.K2_ActivateAbility`
  (bind _returnvalue (`self.GetAbilitySystemComponentFromActorInfo`))
  (bind _asgas_tarea_3character (cast `GAS_Tarea3Character` (`self.GetAvatarActorFromActorInfo`)))
  (if (`GAS_Tarea3Character.IsAttacking` _asgas_tarea_3character)
    (set `GAS_Tarea3Character.IsAttacking` false _asgas_tarea_3character)
    (`self.K2_EndAbility`)
    (else
      (set `GAS_Tarea3Character.IsAttacking` true _asgas_tarea_3character)
      (`AbilitySystemComponent.BP_ApplyGameplayEffectSpecToTarget` _returnvalue (`AbilitySystemComponent.MakeOutgoingSpec` _returnvalue "/Game/Tarea/GE_Protect.GE_Protect_C" 0.0 (`AbilitySystemComponent.MakeEffectContext` _returnvalue)) _returnvalue)
      (`AbilityTask_PlayMontageAndWait.CreatePlayMontageAndWaitProxy` "None" "/Game/Tarea/AM_Protect.AM_Protect" (`self.Anim Speed`)
        (:`OnCompleted`
          (bind _asgas_tarea_3character_2 (cast `GAS_Tarea3Character` (`self.GetAvatarActorFromActorInfo`)))
          (set `GAS_Tarea3Character.IsAttacking` false _asgas_tarea_3character_2)
          (`self.K2_EndAbility`))))))