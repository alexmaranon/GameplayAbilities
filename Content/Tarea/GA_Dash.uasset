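; GA_Dash is a Gameplay Ability that dashes the BP_Knight avatar forward.
; When CanDash is set, it calls the knight's DashUI, launches it horizontally along its forward vector, calls PlayAnimMontage and spawns a DirectionalBurst effect facing that direction.
; Cooldown uses the CanDash flag and a DashCD delay rather than a cooldown effect, so the ability ends only after the delay restores the flag.
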(event `self.K2_ActivateAbility`
  (bind _returnvalue (`self.GetAvatarActorFromActorInfo`))
  (bind (_returnvalue_x _returnvalue_y) (`KismetMathLibrary.BreakVector` (* (`Actor.GetActorForwardVector` (`self.GetAvatarActorFromActorInfo`)) 8000.0)))
  (if (`self.CanDash`)
    (set `self.CanDash` false)
    (bind _asbp_knight (cast `/Game/Tarea/BP_Knight` (`self.GetAvatarActorFromActorInfo`)))
    (`/Game/Tarea/BP_Knight.DashUI` _asbp_knight)
    (`Character.LaunchCharacter` _asbp_knight (`KismetMathLibrary.MakeVector` _returnvalue_x _returnvalue_y) false false)
    (`Character.PlayAnimMontage` _asbp_knight null 1.0 "None")
    (`NiagaraFunctionLibrary.SpawnSystemAtLocation` "/Niagara/DefaultAssets/Templates/Systems/DirectionalBurst.DirectionalBurst" (`Actor.K2_GetActorLocation` _returnvalue) (`KismetMathLibrary.Conv_VectorToRotator` (`Actor.GetActorForwardVector` _returnvalue)) (0.9 2.0 2.0))
    (`KismetSystemLibrary.Delay` (`self.DashCD`))
    (set `self.CanDash` true)
    (`self.K2_EndAbility`)))