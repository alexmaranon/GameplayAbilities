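; BP_Knight is the Knight Blueprint that feeds health and dash cooldown to the main HUD.
; Every Tick it reads a gameplay attribute from its ASC and passes it to HUD_Main as current health, with a hardcoded maximum.
; DashUI plays a Timeline from the start, sending its track value to the HUD's dash cooldown on each update.
; Both paths repeat the player controller and HUD casts instead of caching them.
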(event `self.ReceiveTick`
  (params (DeltaSeconds :type "Float (single-precision)"))
  (`parent.ReceiveTick` DeltaSeconds)
  (bind _aspc_character (cast `/Game/Tarea/PC_Character` (`GameplayStatics.GetPlayerController` 0)))
  (bind _ashud_main (cast `/Game/Tarea/HUD_Main` (`PlayerController.GetHUD` _aspc_character)))
  (`/Game/Tarea/HUD_Main.SetHealth` _ashud_main (`.ReturnValue` (`AbilitySystemComponent.GetGameplayAttributeValue` (`self.ASC`) (struct :`AttributeName` "Health" :`Attribute` "/Script/GAS_Tarea3.CoreAttributeSet:Health" :`AttributeOwner` "/Script/CoreUObject.Class'/Script/GAS_Tarea3.CoreAttributeSet'"))) 200.0))

(event `DashUI`
  ;[1 1 1] Los Casteos deberían de guardarse pero está hecho a prisa
  (bind (_direction _newtrack_0) (`Timeline|Timeline` :!via `PlayFromStart`)
    (:`Update`
      (bind _aspc_character (cast `/Game/Tarea/PC_Character` (`GameplayStatics.GetPlayerController` 0)))
      (bind _ashud_main (cast `/Game/Tarea/HUD_Main` (`PlayerController.GetHUD` _aspc_character)))
      (`/Game/Tarea/HUD_Main.DashCD` _ashud_main _newtrack_0))))

(fn `UserConstructionScript`
  (`parent.UserConstructionScript`))